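; BP_Proyectile is a hazard projectile that respawns the player when it touches the ball pawn.
; Tick moves it along its forward vector at MoveSpeed, scaled by delta time and without sweep.
; Sphere1 overlap checks for BP_BallPawn and calls RespawnPlayer on BP_BallGameMode.
; The SpeedBoost event and the Sphere overlap are empty, leaving the timed speed-multiplier and reset logic disconnected.
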(event OnComponentBeginOverlap(Sphere)
  (params (OverlappedComponent :type Primitive%20Component%20Object%20Reference) (OtherActor :type Actor%20Object%20Reference) (OtherComp :type Primitive%20Component%20Object%20Reference) (OtherBodyIndex :type Integer) (bFromSweep :type Boolean) (SweepResult :type Hit%20Result%20Structure%20%28by%20ref%29)))

(event OnComponentBeginOverlap(Sphere1)
  (params (OverlappedComponent :type Primitive%20Component%20Object%20Reference) (OtherActor :type Actor%20Object%20Reference) (OtherComp :type Primitive%20Component%20Object%20Reference) (OtherBodyIndex :type Integer) (bFromSweep :type Boolean) (SweepResult :type Hit%20Result%20Structure%20%28by%20ref%29))
  (Utilities|Casting|CastToBP_BallPawn OtherActor)
  (bind _asbp_ball_game_mode (Utilities|Casting|CastToBP_BallGameMode (Game|GetGameMode)))
  (Default|RespawnPlayer _asbp_ball_game_mode))

(event EventTick
  (params (DeltaSeconds :type Float%20%28single-precision%29))
  (Transformation|SetActorLocation (+ (* (* DeltaSeconds (Variables|Default|GetMoveSpeed)) (Transformation|GetActorForwardVector)) (Transformation|GetActorLocation)) false false))

(event EventSpeedBoost
  (params (Multiplier :type Float%20%28double-precision%29) (Duration :type Float%20%28double-precision%29)))

(event EventBeginPlay
  (Variables|Default|SetInitialMoveSpeed (Variables|Default|GetMoveSpeed)))

(fn ConstructionScript)