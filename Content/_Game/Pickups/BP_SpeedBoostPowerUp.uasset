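; Speed boost power-up pickup that grants a boost to actors overlapping its Box component.
; Overlapping actors that implement BPI_SpeedBoostable receive SpeedBoostMessage with the pickup's Multiplier and Duration, leaving the boost itself to the receiver.
; It then spawns the PS_SpeedBoost effect and plays the speed-up cue at its location, alongside an extra sound call with no sound set.
; The graph never destroys or disables the pickup.
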(event OnComponentBeginOverlap(Box)
  (params (OverlappedComponent :type Primitive%20Component%20Object%20Reference) (OtherActor :type Actor%20Object%20Reference) (OtherComp :type Primitive%20Component%20Object%20Reference) (OtherBodyIndex :type Integer) (bFromSweep :type Boolean) (SweepResult :type Hit%20Result%20Structure%20%28by%20ref%29))
  (if (Utilities|DoesObjectImplementInterface OtherActor "/Game/_Game/Interfaces/BPI_SpeedBoostable.BPI_SpeedBoostable_C")
    (Class|BPISpeedBoostable|SpeedBoost(Message) OtherActor (Variables|Default|GetMultiplier) (Variables|Default|GetDuration))
    (Audio|PlaySoundatLocation 0 (Transformation|GetActorLocation) "0, 0, 0" 1.0 1.0 0.0 0 0 0 0)
    (Niagara|SpawnSystematLocation "/Game/_Game/Particles/PS_SpeedBoost.PS_SpeedBoost" (Transformation|GetActorLocation))
    (Audio|PlaySoundatLocation "/Game/_Game/Audio/SpeedUpSound_Cue.SpeedUpSound_Cue" (Transformation|GetActorLocation) "0, 0, 0" 1.0 1.0 0.0 0 0 0 0)))

(event EventBeginPlay)

(event Collision|EventActorBeginOverlap
  (params (OtherActor :type Actor%20Object%20Reference)))

(event EventTick
  (params (DeltaSeconds :type Float%20%28single-precision%29)))

(fn ConstructionScript)