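; Player pawn for the Bounce Ball Challenge game: a physics sphere the player rolls and launches through Enhanced Input.
; Move input applies normalized torque to roll the sphere, with top speed set by capping its angular velocity.
; Launch zeroes velocity, then applies an impulse along the held move direction plus a vertical hop, gated by a cooldown.
; SpeedBoost temporarily multiplies the angular velocity cap and plays a particle effect, using a retriggerable delay.
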(event Input|EnhancedActionEvents|EnhancedInputActionIA_Move
  (params (ActionValue :type Vector%202D%20Structure) (ElapsedSeconds :type Float%20%28double-precision%29) (TriggeredSeconds :type Float%20%28double-precision%29) (InputAction :type Input%20Action%20Object%20Reference :default "/Game/_Game/Input/IA_Move.IA_Move"))
  (Class|PrimitiveComponent|AddTorqueinRadians (Variables|Default|GetSphere) (Math|Conversions|ToVector(Vector2D) (* (Math|Vector2D|Normalize2D (Math|Vector2D|MakeVector2D (* (.x ActionValue) -1.0) (.y ActionValue))) (Variables|Default|GetRollTorque))) "None" false))

(event Input|EnhancedActionEvents|EnhancedInputActionIA_Launch
  (params (ActionValue :type Boolean) (ElapsedSeconds :type Float%20%28double-precision%29) (TriggeredSeconds :type Float%20%28double-precision%29) (InputAction :type Input%20Action%20Object%20Reference :default "/Game/_Game/Input/IA_Launch.IA_Launch"))
  (bind _returnvalue (Input|EnhancedActionValues|GetIA_Move))
  (bind _returnvalue_2 (Math|Vector2D|MakeVector2D (.y _returnvalue) (.x _returnvalue)))
  (bind _returnvalue_3 (Math|Vector2D|Normalize2D _returnvalue_2))
  (if (Variables|Default|GetIsLaunchReady)
    (Variables|Default|SetIsLaunchReady false)
    (Class|PrimitiveComponent|SetAllPhysicsLinearVelocity (Variables|Default|GetSphere) "0, 0, 0" false)
    (Physics|AddImpulse (Variables|Default|GetSphere) (* (Math|Vector|MakeVector (.x _returnvalue_3) (.y _returnvalue_3) (Variables|Default|GetVerticalHop)) (Variables|Default|GetLaunchStrenght)) "None" false)
    (Utilities|FlowControl|Delay (Variables|Default|GetLaunchCooldown))
    (Variables|Default|SetIsLaunchReady true)))

(event EventBeginPlay
  (bind _asplayer_controller (Utilities|Casting|CastToPlayerController (Pawn|GetController)))
  (Utilities|IsValid (PlayerController|LocalPlayerSubsystems|GetEnhancedInputLocalPlayerSubsystem _asplayer_controller)
    (:Is%20Valid
      (Input|AddMappingContext (PlayerController|LocalPlayerSubsystems|GetEnhancedInputLocalPlayerSubsystem _asplayer_controller) "/Game/_Game/Input/IMC_Ball.IMC_Ball" 0 "(bIgnoreAllPressedKeysUntilRelease=True,bForceImmediately=False,bNotifyUserSettings=False)")
      (Class|PrimitiveComponent|SetPhysicsMaxAngularVelocityinRadians (Variables|Default|GetSphere) (Variables|Default|GetMaxAngularVelocity) false "None"))))

(event EventSpeedBoost
  (params (Multiplier :type Float%20%28double-precision%29) (Duration :type Float%20%28double-precision%29))
  (Class|PrimitiveComponent|SetPhysicsMaxAngularVelocityinRadians (Variables|Default|GetSphere) (* Multiplier (Variables|Default|GetMaxAngularVelocity)) false "None") ; Speed Up
  (Components|Activation|Activate (Variables|Default|GetSpeedBoostPS) false)
  (Utilities|FlowControl|RetriggerableDelay Duration) ; Wait
  (Class|PrimitiveComponent|SetPhysicsMaxAngularVelocityinRadians (Variables|Default|GetSphere) (Variables|Default|GetMaxAngularVelocity) false "None") ; Reset Speed
  (Components|Activation|Deactivate (Variables|Default|GetSpeedBoostPS)))

(fn ConstructionScript)