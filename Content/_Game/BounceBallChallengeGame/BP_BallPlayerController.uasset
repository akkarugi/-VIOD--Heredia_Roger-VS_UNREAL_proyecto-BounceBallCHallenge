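; Player controller for the bounce ball challenge game, handling HUD, game-level inputs and the win screen.
; On BeginPlay it adds the player info widget and the IMC_BallGame Enhanced Input mapping context.
; Reload, respawn and quit actions cast to BP_BallGameMode, which performs the reload and respawn, while quit exits the game directly.
; The Win event shows the win screen widget and disables input on the player pawn.
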(event Custom|Win
  (Development|PrintString "win")
  (bind _returnvalue (UserInterface|CreateWidget "/Game/_Game/UI/WBP_WinScreen.WBP_WinScreen_C" self))
  (UserInterface|Viewport|AddtoViewport _returnvalue 0)
  (Input|DisableInput (Game|Player|GetPlayerPawn 0) self))

(event Input|EnhancedActionEvents|EnhancedInputActionIA_ReloadLeve
  (params (ActionValue :type Boolean) (ElapsedSeconds :type Float%20%28double-precision%29) (TriggeredSeconds :type Float%20%28double-precision%29) (InputAction :type Input%20Action%20Object%20Reference :default "/Game/_Game/Input/IA_ReloadLeve.IA_ReloadLeve"))
  (bind _asbp_ball_game_mode (Utilities|Casting|CastToBP_BallGameMode (Game|GetGameMode)))
  (Default|ReloadLevel _asbp_ball_game_mode))

(event Input|EnhancedActionEvents|EnhancedInputActionIA_QuitGame
  (params (ActionValue :type Boolean) (ElapsedSeconds :type Float%20%28double-precision%29) (TriggeredSeconds :type Float%20%28double-precision%29) (InputAction :type Input%20Action%20Object%20Reference :default "/Game/_Game/Input/IA_QuitGame.IA_QuitGame"))
  (Utilities|Casting|CastToBP_BallGameMode (Game|GetGameMode))
  (Game|QuitGame 0 "Quit" false))

(event Input|EnhancedActionEvents|EnhancedInputActionIA_Respawn
  (params (ActionValue :type Boolean) (ElapsedSeconds :type Float%20%28double-precision%29) (TriggeredSeconds :type Float%20%28double-precision%29) (InputAction :type Input%20Action%20Object%20Reference :default "/Game/_Game/Input/IA_Respawn.IA_Respawn"))
  (bind _asbp_ball_game_mode (Utilities|Casting|CastToBP_BallGameMode (Game|GetGameMode)))
  (Default|RespawnPlayer _asbp_ball_game_mode))

(event EventBeginPlay
  (bind _returnvalue (UserInterface|CreateWidget "/Game/_Game/UI/WBP_PlayerInfo.WBP_PlayerInfo_C" self))
  (UserInterface|Viewport|AddtoViewport _returnvalue 0)
  (Input|AddMappingContext (PlayerController|LocalPlayerSubsystems|GetEnhancedInputLocalPlayerSubsystem self) "/Game/_Game/Input/IMC_BallGame.IMC_BallGame" 0 "(bIgnoreAllPressedKeysUntilRelease=True,bForceImmediately=False,bNotifyUserSettings=False)"))

(fn ConstructionScript)